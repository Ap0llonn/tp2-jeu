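; Manager Blueprint that controls the visibility of maze walls in the world, caching every BPI_Visible actor on BeginPlay.
; ShuffleWalls loops once per cached actor, toggling a random pick unless a separately randomized BP_Wall pick has the "Maze" Id.
; GetNumberOfWall supplies the random upper bound as array length minus -1, which exceeds the last index.
; RenderMaze reveals hidden walls whose Id matches the given ChestId.
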(event EventBeginPlay
  (bind _outactors (Actor|GetAllActorswithInterface "/Game/Features/MazeVisibilty/BPI_Visible.BPI_Visible_C"))
  (Variables|Default|SetVisibleObjects _outactors))

(fn ConstructionScript)

(fn ShuffleWalls
  (bind _numberofwall (CallFunction|GetNumberOfWall))
  (for _array_element (Variables|Default|GetVisibleObjects)
    (bind _asbpi_visible (Utilities|Casting|CastToBPI_Visible (Utilities|Array|Get(acopy) (Variables|Default|GetVisibleObjects) (Math|Random|RandomIntegerinRange 0 _numberofwall))))
    (bind _asbp_wall (Utilities|Casting|CastToBP_Wall (Utilities|Array|Get(acopy) (Variables|Default|GetVisibleObjects) (Math|Random|RandomIntegerinRange 0 _numberofwall))))
    (if (not (== "Maze" (Variables|/Game/World/BP_Wall.BP_Wall_C|GetId _asbp_wall)))
      (Default|ToggleVisibility _asbpi_visible))))

(fn GetNumberOfWall
  (return (- (Utilities|Array|Length (Variables|Default|GetVisibleObjects)) -1)))

(fn RenderMaze
  (params (ChestId :type Name))
  (for _array_element (Variables|Default|GetVisibleObjects)
    (bind _asbp_wall (Utilities|Casting|CastToBP_Wall _array_element))
    (if (== ChestId (Variables|/Game/World/BP_Wall.BP_Wall_C|GetId _asbp_wall))
      (if (not (Variables|/Game/World/BP_Wall.BP_Wall_C|GetIsVisible _asbp_wall))
        (Default|ToggleVisibility _asbp_wall)))))