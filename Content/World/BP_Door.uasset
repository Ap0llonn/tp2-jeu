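; BP_Door is an interactable hinged door that opens and closes, or stays shut while locked.
; Interact on a locked door casts the player to BP_FirstPersonCharacter and briefly shows a locked message through its UserWidget.
; Otherwise it toggles IsOpen and plays or reverses a single timeline, whose update lerps the Hinge's relative rotation between the DoorClose and DoorOpen rotators.
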(event EventInteract
  (if (Variables|Default|GetIsLocked)
    (bind _asbp_first_person_character (Utilities|Casting|CastToBP_FirstPersonCharacter (Game|GetPlayerCharacter 0)))
    (Default|SetText (Variables|/Game/FirstPerson/Blueprints/BP_FirstPersonCharacter.BP_FirstPersonCharacter_C|GetUserWidget _asbp_first_person_character) "The door is locked" 1.0)
    (elif (Variables|Default|GetIsOpen)
      (Variables|Default|SetIsOpen false)
      (bind _newtrack_0 (Timeline|TL_DoorAnimation Reverse)
        (:Update
          (Transformation|SetRelativeRotation (Variables|Default|GetHinge) (Math|Rotator|Lerp(Rotator) (Variables|Default|GetDoorClose) (Variables|Default|GetDoorOpen) _newtrack_0) false false)))
      (else
        (Variables|Default|SetIsOpen true)
        (Timeline|TL_DoorAnimation Play)))))

(fn ConstructionScript)