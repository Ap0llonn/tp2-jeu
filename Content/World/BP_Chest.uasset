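; Interactable chest that can be claimed once, rewarding the first-person player and revealing a maze.
; On interact, it asks the visibility manager to render the maze for its ChestId, if one is set.
; It then marks itself claimed, turns off its point light, adds a chest to the player character and swings the lid hinge open with a timeline-driven rotation lerp.
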(event EventInteract
  (if (not (Variables|Default|GetIsClaimed))
    (CallFunction|PlaceMaze)
    (CallFunction|OpenChest)
    (bind _newtrack_0 (Timeline|TL_OpenChest Play)
      (:Update
        (Transformation|SetRelativeRotation (Variables|Default|GetChest_Hinge) (Math|Rotator|Lerp(Rotator) (Variables|Default|GetCloseRotation) (Variables|Default|GetOpenRotation) _newtrack_0) false false)))))

(fn ConstructionScript)

(fn OpenChest
  (Variables|Default|SetIsClaimed true)
  (Rendering|Components|Light|SetIntensity (Variables|Default|GetPointLight) 0.0)
  (bind _asbp_first_person_character (Utilities|Casting|CastToBP_FirstPersonCharacter (Game|GetPlayerCharacter 0)))
  (Default|AddChest _asbp_first_person_character))

(fn PlaceMaze
  (bind _chestid (Variables|Default|GetChestId))
  (if (not (== "None" _chestid))
    (bind _returnvalue (Actor|GetActorOfClass "/Game/World/BP_VisibiltyManager.BP_VisibiltyManager_C"))
    (Default|RenderMaze _returnvalue _chestid)))